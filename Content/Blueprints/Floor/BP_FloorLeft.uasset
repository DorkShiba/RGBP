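; BP_FloorLeft is a floor piece that scatters ten building components at random on BeginPlay to vary its scenery.
; SetSize gives each building a random footprint and height, but the values stored in BuildingSize are rolled separately from the applied scale.
; SetLocation randomizes X and Y within the floor at a fixed height, insetting both axes by the stored X size alone.
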(event `self.ReceiveBeginPlay`
  (`parent.ReceiveBeginPlay`)
  (bind _output_get (set `self.arrBuildings` (`|MakeArray` (`self.Building1`) (`self.Building2`) (`self.Building3`) (`self.Building4`) (`self.Building5`) (`self.Building6`) (`self.Building7`) (`self.Building8`) (`self.Building9`) (`self.Building10`))))
  (for _array_element _output_get
    (`self.SetSize` _array_element)
    (`self.SetLocation` _array_element)))

(fn `SetLocation`
  (params (targetBuilding :type "SceneComponent Object Reference"))
  (locals (xGap :type "Float (double-precision)") (yGap :type "Float (double-precision)") (xLoc :type "Float (double-precision)" :default 0.0) (yLoc :type "Float (double-precision)" :default 0.0))
  (set `local.xGap` (* (`|GetArrayItem` (`self.buildingSize`)) 50.0))
  (set `local.yGap` (* (`|GetArrayItem` (`self.buildingSize`)) 50.0))
  (bind _output_get (set `local.xLoc` (`KismetMathLibrary.RandomFloatInRange` (+ -50.0 (`local.xGap`)) (- 50.0 (`local.xGap`)))))
  (bind _output_get_2 (set `local.yLoc` (`KismetMathLibrary.RandomFloatInRange` (+ -50.0 (`local.yGap`)) (- 50.0 (`local.yGap`)))))
  (`SceneComponent.K2_SetRelativeLocation` targetBuilding (`KismetMathLibrary.MakeVector` _output_get _output_get_2 100.0) false false))

(fn `SetSize`
  (params (targetBuilding :type "StaticMeshComponent Object Reference"))
  (bind _returnvalue (`KismetMathLibrary.RandomFloatInRange` 0.01 0.2))
  (bind _returnvalue_2 (`KismetMathLibrary.RandomFloatInRange` 0.01 0.2))
  (bind _returnvalue_3 (`KismetMathLibrary.RandomFloatInRange` 0.1 3.0))
  (`KismetArrayLibrary.Array_Set` (`self.buildingSize`) 0 _returnvalue)
  (`KismetArrayLibrary.Array_Set` (`self.buildingSize`) 1 _returnvalue_2)
  (`KismetArrayLibrary.Array_Set` (`self.buildingSize`) 2 _returnvalue_3)
  (`SceneComponent.SetRelativeScale3D` targetBuilding (`KismetMathLibrary.MakeVector` _returnvalue _returnvalue_2 _returnvalue_3)))

(fn `UserConstructionScript`
  (`parent.UserConstructionScript`))